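; Base Gameplay Ability for melee attacks, which plays an attack montage using the avatar's equipped weapon from BP_WeaponsManagerComponent.
; On authority, HitScan Start and End gameplay events open and close the weapon's hit scan, passing it a damage effect spec with set-by-caller magnitude.
; The ability ends when the montage finishes or is interrupted, or if setup is invalid, and always stops the scan.
; Children can override MontageStarted.
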(event `self.K2_ActivateAbility`
  (bind _returnvalue (`Actor.GetComponentByClass` (`self.GetAvatarActorFromActorInfo`) "/Game/Weapons/BP_WeaponsManagerComponent.BP_WeaponsManagerComponent_C"))
  (`/Engine/EditorBlueprintResources/StandardMacros.IsValid` _returnvalue
    (:`Is Valid`
      (bind _equippedweapon (`/Game/Weapons/BP_WeaponsManagerComponent.EquippedWeapon` _returnvalue)
        (:`then`
          (set `self.EquippedWeapon` _equippedweapon)
          (bind _attackmontage (`self.AttackMontage`)
            (:`then`
              (`AbilityTask_PlayMontageAndWait.CreatePlayMontageAndWaitProxy` "None" _attackmontage 1.0 "None" true 1.0 0.0 true
                (:`then`
                  (`self.MontageStarted`)
                  (`self.K2_HasAuthority`
                    (:`True`
                      (`AbilityTask_WaitGameplayEvent.WaitGameplayEvent` (struct :`TagName` "Event.HitScan.Start") null
                        (:`then`
                          (`AbilityTask_WaitGameplayEvent.WaitGameplayEvent` (struct :`TagName` "Event.HitScan.End") null
                            (:`EventReceived`
                              (`self.HandleHitScanEnd`))))
                        (:`EventReceived`
                          (`self.HandleHitScanStart`))))))
                (:`OnCompleted`
                  (`self.K2_EndAbility` :!label _label))
                (:`OnInterrupted`
                  (goto _label))
                (:`OnCancelled`
                  (goto _label))))
            (:`else`
              (`self.K2_EndAbility` :!label _label_2))))
        (:`else`
          (goto _label_2))))
    (:`Is Not Valid`
      (goto _label_2))))

(event `HandleHitScanStart`
  ; Hit Scan Events
  (bind _equippedweapon (`self.EquippedWeapon`)
    (:`then`
      (bind _returnvalue (`AbilitySystemBlueprintLibrary.AssignTagSetByCallerMagnitude` (`self.MakeOutgoingGameplayEffectSpec` (`self.DamageEffectClass`)) (struct :`TagName` "Data.Damage") (`self.DamageMagnitude`)))
      (`/Game/Weapons/BP_Weapon_Base.HitScanStart` _equippedweapon _returnvalue))
    (:`else`)))

(event `HandleHitScanEnd`
  ; Hit Scan Events
  (bind _equippedweapon (`self.EquippedWeapon`)
    (:`then`
      (`/Game/Weapons/BP_Weapon_Base.HitScanEnd` _equippedweapon))
    (:`else`)))

(event `MontageStarted`
  ; Override in child
)

(event `self.K2_OnEndAbility`
  (params (bWasCancelled :type Boolean))
  (`self.HandleHitScanEnd`))