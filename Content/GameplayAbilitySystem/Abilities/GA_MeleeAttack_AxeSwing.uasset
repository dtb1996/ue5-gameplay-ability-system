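; Gameplay ability for a melee axe swing using the avatar's equipped weapon from its weapons manager component, ending at once if none exists.
; It plays the swing montage and, on authority only, waits for hit-scan start and end gameplay events to open and close the weapon's hit scan.
; The start event hands the weapon an instant damage effect spec with set-by-caller magnitude.
; Any montage exit ends the ability, which also stops the hit scan.
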(event `self.K2_ActivateAbility`
  (bind _returnvalue (`Actor.GetComponentByClass` (`self.GetAvatarActorFromActorInfo`) "/Game/Weapons/BP_WeaponsManagerComponent.BP_WeaponsManagerComponent_C"))
  (`/Engine/EditorBlueprintResources/StandardMacros.IsValid` _returnvalue
    (:`Is Valid`
      (bind _equippedweapon (`/Game/Weapons/BP_WeaponsManagerComponent.EquippedWeapon` _returnvalue)
        (:`then`
          (set `self.EquippedWeapon` _equippedweapon)
          (`AbilityTask_PlayMontageAndWait.CreatePlayMontageAndWaitProxy` "None" "/Game/Characters/Mixamo/Retargets/AM_MeleeAttack_AxeSwing.AM_MeleeAttack_AxeSwing" 1.0 "None" true 1.0 0.0 true
            (:`then`
              (`self.K2_HasAuthority`
                (:`True`
                  (`AbilityTask_WaitGameplayEvent.WaitGameplayEvent` (struct :`TagName` "Event.HitScan.Start") null
                    (:`then`
                      (`AbilityTask_WaitGameplayEvent.WaitGameplayEvent` (struct :`TagName` "Event.HitScan.End") null
                        (:`EventReceived`
                          (bind _equippedweapon_2 (`self.EquippedWeapon`)
                            (:`then`
                              (`/Game/Weapons/BP_Weapon_Base.HitScanEnd` _equippedweapon_2))
                            (:`else`)))))
                    (:`EventReceived`
                      (bind _equippedweapon_3 (`self.EquippedWeapon`)
                        (:`then`
                          (bind _returnvalue_2 (`AbilitySystemBlueprintLibrary.AssignTagSetByCallerMagnitude` (`self.MakeOutgoingGameplayEffectSpec` "/Game/GameplayAbilitySystem/Effects/GE_Damage_Instant.GE_Damage_Instant_C") (struct :`TagName` "Data.Damage") -34.0))
                          (`/Game/Weapons/BP_Weapon_Base.HitScanStart` _equippedweapon_3 _returnvalue_2))
                        (:`else`)))))))
            (:`OnCompleted`
              (`self.K2_EndAbility` :!label _label))
            (:`OnInterrupted`
              (goto _label))
            (:`OnCancelled`
              (goto _label))))
        (:`else`
          (`self.K2_EndAbility` :!label _label_2))))
    (:`Is Not Valid`
      (goto _label_2))))

(event `self.K2_OnEndAbility`
  (params (bWasCancelled :type Boolean))
  (bind _equippedweapon (`self.EquippedWeapon`)
    (:`then`
      (`/Game/Weapons/BP_Weapon_Base.HitScanEnd` _equippedweapon))
    (:`else`)))